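; Player Blueprint for an idle battler that owns random stats, a battle countdown and the game's menu flow.
; BeginPlay rolls six stats and creates the HUD widgets, which click events and Escape swap, asking for a name when none is set.
; Delay-gated Tick logic counts down battle time, refills it shortened by Speed, and uses a DoOnce to count wins.
; Q boosts Speed, and the win count prints every tick as debug output.
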(event Custom|ClickedSettings
  ;[1 1 1] Changing HUDs
  (Widget|RemovefromParent (Variables|Default|GetMainMenuHUD))
  (UserInterface|Viewport|AddtoViewport (Variables|Default|GetSettingsHUD) 0))

(event Custom|ClickedPlayButton
  ;[1 1 1] Changing HUDs
  (if (Variables|Default|GetHaveName)
    (Widget|RemovefromParent (Variables|Default|GetMainMenuHUD))
    (UserInterface|Viewport|AddtoViewport (Variables|Default|GetGameHUD) 0)
    (else
      (Widget|RemovefromParent (stale EventBeginPlay _output_get))
      (UserInterface|Viewport|AddtoViewport (Variables|Default|GetNameInsertHUD) 0))))

(event Custom|ClickedConfirmButton
  ;[1 1 1] Changing HUDs
  (Widget|RemovefromParent (Variables|Default|GetNameInsertHUD))
  (UserInterface|Viewport|AddtoViewport (Variables|Default|GetGameHUD) 0))

(event Custom|ClickedBackSettings
  ;[1 1 1] Changing HUDs
  (Widget|RemovefromParent (Variables|Default|GetSettingsHUD))
  (UserInterface|Viewport|AddtoViewport (Variables|Default|GetMainMenuHUD) 0))

(event Custom|ClickedMenu
  ;[1 1 1] Back To Menu
  (if (Variables|Default|GetInGame)
    (Widget|RemovefromParent (Variables|Default|GetGameHUD))
    (UserInterface|Viewport|AddtoViewport (Variables|Default|GetMainMenuHUD) 0)))

(event EventTick
  (params (DeltaSeconds :type Float%20%28single-precision%29))
  (Utilities|FlowControl|Sequence
    (:then_0
      ;[1 1 1] BattleCountDownTimer
      (if (Variables|Default|GetInGame)
        (Utilities|FlowControl|Delay 1.0)
        (Variables|Default|SetPlayerBattleTime (- (Variables|Default|GetPlayerBattleTime) 1.0))))
    (:then_1
      (if (<= (Variables|Default|GetPlayerBattleTime) 0.0)
        (Utilities|FlowControl|Delay 1.0)
        (Variables|Default|SetPlayerBattleTime (- (Variables|Default|GetConstructBattleTime) (* (Variables|Default|GetPlayerSpeed) 0.1)))))
    (:then_2
      (if (<= (Variables|Default|GetPlayerBattleTime) 1.0)
        (Utilities|FlowControl|Delay 2.0)
        (Utilities|FlowControl|DoOnce true :!label _label
          (:Completed
            (Variables|Default|SetBattlesWon (+ (Variables|Default|GetBattlesWon) 1))))
        (else
          (goto _label Reset))))
    (:then_3
      (Development|PrintString (Utilities|String|ToString(Integer) (Variables|Default|GetBattlesWon)) true true "(R=0.000000,G=0.660000,B=1.000000,A=1.000000)" 0.0))))

(event EventBeginPlay
  (bind _returnvalue (Math|Random|RandomFloatinRange 0.0 6.0))
  (Utilities|FlowControl|Sequence
    (:then_0
      ;[1 1 1] Random Stats
      (Variables|Default|SetPlayerDefence _returnvalue)
      (Variables|Default|SetPlayerSpeed _returnvalue)
      (Variables|Default|SetPlayerDamage _returnvalue)
      (Variables|Default|SetPlayerGreed _returnvalue)
      (Variables|Default|SetPlayerMagic _returnvalue)
      (Variables|Default|SetPlayerLuck _returnvalue))
    (:then_1
      ;[1 1 1] Changing HUDs
      (bind _returnvalue_2 (UserInterface|CreateWidget "/Game/Blueprints/NameInputHUD.NameInputHUD_C"))
      (bind _returnvalue_3 (UserInterface|CreateWidget "/Game/Blueprints/GameHUD.GameHUD_C"))
      (bind _returnvalue_4 (UserInterface|CreateWidget "/Game/Blueprints/MainMenuHUD.MainMenuHUD_C"))
      (bind _returnvalue_5 (UserInterface|CreateWidget "/Game/Blueprints/SettingsHUD.SettingsHUD_C"))
      (bind _output_get (Variables|Default|SetMainMenuHUD _returnvalue_4))
      (UserInterface|Viewport|AddtoViewport _output_get 0)
      (Variables|Default|SetGameHUD _returnvalue_3)
      (Variables|Default|SetNameInsertHUD _returnvalue_2)
      (Variables|Default|SetSettingsHUD _returnvalue_5))))

(event Input|KeyboardEvents|Escape
  (params (Key :type Key%20Structure :default "AnyKey"))
  (:Pressed
    ;[1 1 1] Back To Menu
    (if (Variables|Default|GetInGame)
      (Widget|RemovefromParent (Variables|Default|GetGameHUD))
      (UserInterface|Viewport|AddtoViewport (Variables|Default|GetMainMenuHUD) 0))))

(event Input|KeyboardEvents|Q
  (params (Key :type Key%20Structure :default "AnyKey"))
  (:Pressed
    (Variables|Default|SetPlayerSpeed (+ (Variables|Default|GetPlayerSpeed) 2.0))))

(fn ConstructionScript
  (Variables|Default|SetConstructBattleTime (Variables|Default|GetPlayerBattleTime)))